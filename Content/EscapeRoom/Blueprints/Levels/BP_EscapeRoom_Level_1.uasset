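; BP_EscapeRoom_Level_1 is an escape room Blueprint for the first level's code-entry interaction and warning light.
; Releasing a touch on Box while IsActive is set has the game mode open the input code widget.
; SetWarningLight swaps the Light's glass material according to whether IsRight is true.
; Disconnected, never-run logic would cycle hint text through a reused WBP_Hint widget.
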(event OnInputTouchEnd(Box)
  (params (FingerIndex :type ETouchIndex%20Enum :default "Touch1") (TouchedComponent :type Primitive%20Component%20Object%20Reference))
  (if (Variables|Default|GetIsActive)
    (bind _asbp_escape_room_game_mode (Utilities|Casting|CastToBP_EscapeRoom_GameMode (Game|GetGameMode)))
    (Class|EscapeRoomGameMode|OpenInputCodeWitget _asbp_escape_room_game_mode)))

(event EventSetWarningLight
  (params (IsRight :type Boolean))
  (bind _light (Variables|Default|GetLight))
  (if IsRight
    (Rendering|Material|SetMaterial _light 1 "/Game/EscapeRoom/Materials/M_EscapeRoom_warningLight_01_glass_mat_2.M_EscapeRoom_warningLight_01_glass_mat_2")
    (else
      (Rendering|Material|SetMaterial _light 1 "/Game/EscapeRoom/Materials/M_EscapeRoom_warningLight_01_glass_mat_01.M_EscapeRoom_warningLight_01_glass_mat_01"))))

(event Collision|EventActorBeginOverlap
  (params (OtherActor :type Actor%20Object%20Reference)))

(event EventTick
  (params (DeltaSeconds :type Float%20%28single-precision%29)))

(fn ConstructionScript)