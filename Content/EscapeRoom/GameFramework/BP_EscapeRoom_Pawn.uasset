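; Escape room pawn that answers help requests with contextual hint messages.
; From level 1 onward, it enables DialogCollisionComponent on demand to find overlapping EscapeRoom_Level actors and calls ShowHintMessage through I_EscapeRoom_Dialog, then disables the collision.
; Before level 1, or when nothing overlaps, the game mode shows the hint through the same interface.
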(event EventBeginPlay)

(event Collision|EventActorBeginOverlap
  (params (OtherActor :type Actor%20Object%20Reference)))

(event EventTick
  (params (DeltaSeconds :type Float%20%28single-precision%29)))

(event EventOnHelpRequest
  (bind _returnvalue (Game|GetGameMode))
  (bind _dialogcollisioncomponent (Variables|Default|GetDialogCollisionComponent))
  (bind _overlappingactors (Collision|GetOverlappingActors _dialogcollisioncomponent "/Script/EscapeRoomV2.EscapeRoom_Level" :!class /Script/Engine.PrimitiveComponent))
  (bind _asbp_escape_room_game_mode (Utilities|Casting|CastToBP_EscapeRoom_GameMode (Game|GetGameMode)))
  (bind _returnvalue_2 (Class|EscapeRoomGameMode|GetCurrentLevel _asbp_escape_room_game_mode))
  (if (>= _returnvalue_2 1)
    (Collision|SetCollisionEnabled _dialogcollisioncomponent "QueryAndPhysics")
    (if (> (Utilities|Array|Length _overlappingactors) 0)
      (for _array_element _overlappingactors
        (if (Utilities|DoesObjectImplementInterface _array_element "/Script/EscapeRoomV2.I_EscapeRoom_Dialog")
          (Class|IEscapeRoomDialog|ShowHint(Message) _array_element)
          (Collision|SetCollisionEnabled (Variables|Default|GetDialogCollisionComponent) "NoCollision")))
      (else
        (if (Utilities|DoesObjectImplementInterface _returnvalue "/Script/EscapeRoomV2.I_EscapeRoom_Dialog") :!label _label
          (Class|IEscapeRoomDialog|ShowHint(Message) _returnvalue))))
    (else
      (goto _label))))

(fn ConstructionScript)