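; Game mode for an escape room that owns the screen widgets and exposes events to control them and the level lighting.
; On BeginPlay it creates the dark screen, main UI and a hidden input-code widget, which events open and close.
; ToggleGlobalLight flips the dark overlay and sets every DirectionalLight's visibility to its inverse.
; ShowHint lazily creates the hint widget and cycles through the Hints array, wrapping to the start.
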(event EventBeginPlay
  (Utilities|FlowControl|Sequence
    (:then_0
      (bind _returnvalue (UserInterface|CreateWidget "/Game/EscapeRoom/Blueprints/Widgets/WBP_DarkScreen.WBP_DarkScreen_C"))
      (bind _output_get (Variables|Default|SetdarkScreen _returnvalue))
      (UserInterface|Viewport|AddtoViewport _output_get 0))
    (:then_1
      (bind _returnvalue_2 (UserInterface|CreateWidget "/Game/EscapeRoom/Blueprints/Widgets/WBP_UI.WBP_UI_C"))
      (UserInterface|Viewport|AddtoViewport _returnvalue_2 0))
    (:then_2
      (bind _returnvalue_3 (UserInterface|CreateWidget "/Game/EscapeRoom/Blueprints/Widgets/WBP_InputCode.WBP_InputCode_C"))
      (bind _output_get_2 (Variables|Default|SetInputCode_1 _returnvalue_3))
      (UserInterface|Viewport|AddtoViewport _output_get_2 0)
      (Widget|SetVisibility _output_get_2 "Hidden"))))

(event EventTick
  (params (DeltaSeconds :type Float%20%28single-precision%29)))

(event EventToggleGlobalLight
  (bind _darkscreen (Variables|Default|GetdarkScreen))
  (bind _returnvalue (Widget|IsVisible _darkscreen))
  (if _returnvalue
    (Widget|SetVisibility _darkscreen "Hidden")
    (else
      (Widget|SetVisibility _darkscreen "Visible")))
  (bind _outactors (Actor|GetAllActorsOfClass "/Script/Engine.DirectionalLight"))
  (for _array_element _outactors
    (Rendering|SetVisibility (Variables|/Script/Engine.Actor|GetRootComponent _array_element) (not _returnvalue) false)))

(event EventShowHint
  (bind _hintui (Variables|Default|GetHintUI)
    (:then
      (if (Widget|IsVisible (Variables|Default|GetHintUI))
        _
        (else
          (Widget|SetVisibility _hintui "Visible"))))
    (:else
      (bind _returnvalue (UserInterface|CreateWidget "/Game/EscapeRoom/Blueprints/Widgets/WBP_Hint.WBP_Hint_C"))
      (bind _output_get (Variables|Default|SetHintUI _returnvalue))
      (UserInterface|Viewport|AddtoViewport _output_get 0)))
  (Default|PrintText _output_get (Utilities|Array|Get(acopy) (Variables|Default|GetHints) (Variables|Default|GetHintIndex)))
  (bind _result (Math|Integer|IncrementInt (Variables|Default|GetHintIndex))
    (:%20%20
      (if (>= _result (Utilities|Array|Length (Variables|Default|GetHints)))
        (Variables|Default|SetHintIndex 0)))))

(event EventCloseInputCodeWitget
  (Development|PrintString "CLICKED")
  (Widget|SetVisibility (Variables|Default|GetInputCode_1) "Hidden"))

(event EventOpenInputCodeWitget
  (Widget|SetVisibility (Variables|Default|GetInputCode_1) "Visible"))

(fn ConstructionScript)